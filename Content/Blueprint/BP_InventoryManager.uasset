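; BP_InventoryManager is a Blueprint that toggles the inventory screen when the I key is pressed.
; Opening creates a WBP_Inventory widget, handing it a reference to itself and WBP_Item as the item widget class, then shows the cursor, switches to Game and UI input, and ignores look input.
; Closing removes the stored widget, clears the reference, and restores game-only input, hidden cursor and camera look.
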(event Input|KeyboardEvents|I
  (params (Key :type Key%20Structure :default "None"))
  (bind _returnvalue (Game|GetPlayerController 0))
  (bind _returnvalue_2 (Game|GetPlayerController 0))
  (:Pressed
    (Utilities|IsValid (Variables|Default|GetInventoryWidgetRef)
      (:Is%20Valid
        ;[0.15 0.15 0.15 0.5] Inventory 닫기
        (Widget|RemovefromParent (Variables|Default|GetInventoryWidgetRef))
        (Variables|Default|SetInventoryWidgetRef 0)
        (Variables|/Script/Engine.PlayerController|SetbShowMouseCursor _returnvalue_2 false)
        (Input|SetInputModeGameOnly _returnvalue_2 false)
        (Input|SetIgnoreLookInput (Game|GetPlayerController 0) false))
      (:Is%20Not%20Valid
        ;[0.15 0.15 0.15 0.5] Inventory 띄우기
        (bind _returnvalue_3 (UserInterface|CreateWidget "/Game/Blueprint/WBP_Inventory.WBP_Inventory_C" 0 self "/Game/Blueprint/WBP_Item.WBP_Item_C"))
        (UserInterface|Viewport|AddtoViewport _returnvalue_3 0)
        (Variables|Default|SetInventoryWidgetRef _returnvalue_3)
        ;[0.15 0.15 0.15 0.5] 마우스로 UI 조작
        (Variables|/Script/Engine.PlayerController|SetbShowMouseCursor _returnvalue true)
        (Input|SetInputModeGameandUI _returnvalue (Variables|Default|GetInventoryWidgetRef) "DoNotLock" true false)
        (Input|SetIgnoreLookInput (Game|GetPlayerController 0) true)))))

(fn ConstructionScript)